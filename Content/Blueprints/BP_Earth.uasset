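; BP_Earth is the Earth actor in a simulation, moving along a circular orbit around the location where it starts.
; On BeginPlay it caches the PC_Simulation controller, stores the orbit center and draws a temporary debug circle for the path.
; OrbitSpin runs every Tick, placing the actor with sine and cosine of the controller's SimulationTimer, scaled by OrbitRadius and slowed by OrbitSlowed.
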(event `self.ReceiveBeginPlay`
  (bind (_orbitcenter_x _orbitcenter_y) (`KismetMathLibrary.BreakVector` (`self.OrbitCenter`)))
  (`|ExecutionSequence`
    (:`then_0`
      (bind _aspc_simulation (cast `/Game/Blueprints/PC_Simulation` (`GameplayStatics.GetPlayerController` 0)))
      (set `self.PlayerController` _aspc_simulation))
    (:`then_1`
      (set `self.OrbitCenter` (`self.K2_GetActorLocation`)))
    (:`then_2`
      (`KismetSystemLibrary.DrawDebugCircle` (`KismetMathLibrary.MakeVector` _orbitcenter_x _orbitcenter_y) (`self.OrbitRadius`) 2000 (struct :`R` 1.0 :`G` 1.0 :`B` 1.0 :`A` 1.0) 300.0 500.0 (0.0 1.0 0.0) (1.0 0.0 0.0) true)
      (`self.OrbitSpin`))))

(event `self.ReceiveTick`
  (params (DeltaSeconds :type "Float (single-precision)"))
  (`self.OrbitSpin`))

(fn `OrbitSpin`
  (bind _orbitradius (`self.OrbitRadius`))
  (bind (_orbitcenter_x _orbitcenter_y) (`KismetMathLibrary.BreakVector` (`self.OrbitCenter`)))
  (bind _returnvalue (/ (`/Game/Blueprints/PC_Simulation.SimulationTimer` (`self.PlayerController`)) (`self.OrbitSlowed`)))
  (`self.K2_SetActorLocation` (`KismetMathLibrary.MakeVector` (+ _orbitcenter_x (* (`KismetMathLibrary.Sin` _returnvalue) _orbitradius)) (+ _orbitcenter_y (* (`KismetMathLibrary.Cos` _returnvalue) _orbitradius)))))

(fn `UserConstructionScript`)