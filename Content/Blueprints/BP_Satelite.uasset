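; Simulated satellite that is launched by a physics push and visualizes its motion with debug lines.
; When PC_Simulation signals game start, it freezes for a start delay, then pushes its Cone along the up vector with mass-scaled force.
; It marks the launch axis with a long-lived line and records the resulting speed shortly after.
; Each tick it adds a trajectory segment and, unless paused, redraws the current velocity axis.
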(event `self.ReceiveBeginPlay`
  (`|ExecutionSequence`
    (:`then_0`
      (bind _aspawn_simulation (cast `/Game/Blueprints/Pawn_Simulation` (`GameplayStatics.GetPlayerPawn` 0)))
      (set `self.Pawn` _aspawn_simulation))
    (:`then_1`
      (bind _aspc_simulation (cast `/Game/Blueprints/PC_Simulation` (`GameplayStatics.GetPlayerController` 0)))
      (set `self.PlayerController` _aspc_simulation))
    (:`then_2`
      (add `/Game/Blueprints/PC_Simulation.OnGameStarted` (`self.PlayerController`) (delegate `OnGameStarted_Event`)))))

(event `OnGameStarted_Event`
  (bind _startdelay (`self.StartDelay`))
  (bind _cone (`self.Cone`))
  (`self.Freeze`)
  (`/Game/Blueprints/PC_Simulation.OnDelayStarted` (`self.PlayerController`) _startdelay)
  (`KismetSystemLibrary.Delay` _startdelay)
  (`self.UnFreeze`)
  (`PrimitiveComponent.AddForce` _cone (* (`SceneComponent.GetUpVector` _cone) (`self.StartForce`) (`PrimitiveComponent.GetMass` (`self.Cone`))) "None" false)
  (`self.DrawAngleLine` (struct :`G` 1.0 :`A` 1.0) 300.0 true)
  (`KismetSystemLibrary.Delay` 0.2)
  (set `self.StartVelocityLocked` (`KismetMathLibrary.VSize` (`self.GetVelocity`))))

(event `self.ReceiveTick`
  (params (DeltaSeconds :type "Float (single-precision)"))
  (`|ExecutionSequence`
    (:`then_0`
      (`self.DrawTrajectory` DeltaSeconds))
    (:`then_1`
      (if (not (`/Game/Blueprints/PC_Simulation.bGamePaused` (`self.PlayerController`)))
        (`self.DrawAngleLine` (struct :`B` 1.0 :`A` 1.0) (* DeltaSeconds 2.0))))))

(fn `DrawAngleLine`
  (params (Color :type "LinearColor Structure") (Duration :type "Float (double-precision)" :default 300.0) (OnStartVelBased :type Boolean))
  (bind _returnvalue (`self.K2_GetActorLocation`))
  (bind _returnvalue_2 (`self.K2_GetActorLocation`))
  (bind _returnvalue_3 (`KismetMathLibrary.Normal` (`self.GetVelocity`)))
  (bind _returnvalue_4 (`KismetMathLibrary.Normal` (* (`SceneComponent.GetUpVector` (`self.Cone`)) (`self.StartForce`))))
  (if OnStartVelBased
    (`KismetSystemLibrary.DrawDebugLine` (+ _returnvalue_2 (* _returnvalue_4 -1.0 1000000.0)) (+ _returnvalue_2 (* _returnvalue_4 1000000.0)) Color Duration 300.0)
    (else
      (`KismetSystemLibrary.DrawDebugLine` (+ _returnvalue (* _returnvalue_3 -1.0 1000000.0)) (+ _returnvalue (* _returnvalue_3 1000000.0)) Color Duration 300.0))))

(fn `UserConstructionScript`)