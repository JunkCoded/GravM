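; Player pawn for the simulation: a free-fly viewer with Enhanced Input controls for movement, look, speed, pause and level restart.
; Movement offsets the actor along its forward and right vectors by Speed per input event, without sweep or delta-time scaling.
; Speed input changes Speed in proportion to its current value and broadcasts PawnSpeedChanged, which also fires on BeginPlay.
; BeginPlay also caches PC_Simulation, used for pausing, and a BP_Satelite as FocusedSatelite.
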(event `self.ReceiveBeginPlay`
  (`|ExecutionSequence`
    (:`then_0`
      (`self.PawnSpeedChanged` (`self.Speed`)))
    (:`then_1`
      (bind _aspc_simulation (cast `/Game/Blueprints/PC_Simulation` (`GameplayStatics.GetPlayerController` 0)))
      (set `self.PlayerController` _aspc_simulation))
    (:`then_2`
      (bind _returnvalue (`GameplayStatics.GetActorOfClass` "/Game/Blueprints/BP_Satelite.BP_Satelite_C"))
      (set `self.FocusedSatelite` _returnvalue))))

(event `EnhancedInput|/Game/Input/IA_Move`
  (params (ActionValue :type "Vector2D Structure") (ElapsedSeconds :type "Float (double-precision)") (TriggeredSeconds :type "Float (double-precision)") (InputAction :type "InputAction Object Reference" :default "/Game/Input/IA_Move.IA_Move"))
  (bind _speed (`self.Speed`))
  (:`Triggered`
    (`self.K2_SetActorLocation` (+ (`self.K2_GetActorLocation`) (* ActionValue_X (`self.GetActorForwardVector`) _speed) (* ActionValue_Y (`self.GetActorRightVector`) _speed)))))

(event `EnhancedInput|/Game/Input/IA_Look`
  (params (ActionValue :type "Vector2D Structure") (ElapsedSeconds :type "Float (double-precision)") (TriggeredSeconds :type "Float (double-precision)") (InputAction :type "InputAction Object Reference" :default "/Game/Input/IA_Look.IA_Look"))
  (:`Triggered`
    (`self.AddControllerYawInput` ActionValue_X)
    (`self.AddControllerPitchInput` ActionValue_Y)))

(event `EnhancedInput|/Game/Input/IA_Speed`
  (params (ActionValue :type "Float (double-precision)") (ElapsedSeconds :type "Float (double-precision)") (TriggeredSeconds :type "Float (double-precision)") (InputAction :type "InputAction Object Reference" :default "/Game/Input/IA_Speed.IA_Speed"))
  (:`Triggered`
    (bind _output_get (set `self.Speed` (+ (`KismetMathLibrary.FCeil` (* ActionValue (/ (`KismetMathLibrary.Conv_IntToDouble` (`self.Speed`)) 10.0))) (`self.Speed`))))
    (`self.PawnSpeedChanged` _output_get)))

(event `EnhancedInput|/Game/Input/IA_Restart`
  (params (ActionValue :type Boolean) (ElapsedSeconds :type "Float (double-precision)") (TriggeredSeconds :type "Float (double-precision)") (InputAction :type "InputAction Object Reference" :default "/Game/Input/IA_Restart.IA_Restart"))
  (:`Triggered`
    (`GameplayStatics.OpenLevel` (`KismetStringLibrary.Conv_StringToName` (`KismetSystemLibrary.GetObjectName` (`self.GetLevel`))))))

(event `EnhancedInput|/Game/Input/IA_Pause`
  (params (ActionValue :type Boolean) (ElapsedSeconds :type "Float (double-precision)") (TriggeredSeconds :type "Float (double-precision)") (InputAction :type "InputAction Object Reference" :default "/Game/Input/IA_Pause.IA_Pause"))
  (bind _playercontroller (`self.PlayerController`))
  (:`Triggered`
    (`/Game/Blueprints/PC_Simulation.SetPauseGame` _playercontroller (not (`/Game/Blueprints/PC_Simulation.bGamePaused` _playercontroller)) false)))

(fn `UserConstructionScript`)